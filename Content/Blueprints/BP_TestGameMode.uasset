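; BP_TestGameMode is a test game mode that respawns players at spawn markers.
; Its Respawn event takes a controller and, on authority, spawns a BP_PlayerPawn at a random BP_SpawnPos actor, adjusting for collisions, then has the controller possess it.
; Location and rotation each make their own random pick, so they can come from different markers.
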(event Custom|Respawn
  (params (Controller :type Player%20Controller%20Object%20Reference))
  (Utilities|IsValid Controller
    (:Is%20Valid
      (Networking|SwitchHasAuthority
        (:Authority
          (bind _outactors (Actor|GetAllActorsOfClass "/Game/Blueprints/BP_SpawnPos.BP_SpawnPos_C"))
          (bind _returnvalue (Game|SpawnActorfromClass "/Game/Blueprints/BP_PlayerPawn.BP_PlayerPawn_C" (Math|Transform|MakeTransform (Transformation|GetActorLocation (Utilities|Array|Get(acopy) _outactors (Math|Random|RandomInteger (Utilities|Array|Length _outactors)))) (Transformation|GetActorRotation (Utilities|Array|Get(acopy) _outactors (Math|Random|RandomInteger (Utilities|Array|Length _outactors))))) "AdjustIfPossibleButAlwaysSpawn" 0 0))
          (Utilities|IsValid _returnvalue
            (:Is%20Valid
              (Pawn|Possess Controller _returnvalue))))))))

(fn ConstructionScript)