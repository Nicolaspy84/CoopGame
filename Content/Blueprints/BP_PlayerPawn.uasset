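; BP_PlayerPawn is the player pawn Blueprint, handling HUD creation and walk speed setup.
; On BeginPlay, a locally controlled pawn creates crosshair and health widgets and adds them to the viewport.
; The Construction Script applies MaxSpeed to CharacterMovement, then picks a run or walk MaxSpeed from IsRunning, so that pick follows the assignment.
; Similar speed logic in the EventGraph is disconnected and never runs.
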(event EventBeginPlay
  (if (Pawn|IsLocallyControlled)
    (Utilities|FlowControl|Sequence
      (:then_0
        (bind _returnvalue (UserInterface|CreateWidget "/Game/UI/WBP_Crosshair.WBP_Crosshair_C"))
        (UserInterface|Viewport|AddtoViewport _returnvalue 0))
      (:then_1
        (bind _returnvalue_2 (UserInterface|CreateWidget "/Game/Blueprints/WBP_Health.WBP_Health_C"))
        (UserInterface|Viewport|AddtoViewport _returnvalue_2 0)))))

(fn ConstructionScript
  (Variables|/Script/Engine.CharacterMovementComponent|SetMaxWalkSpeed (Variables|Character|GetCharacterMovement) (Variables|Default|GetMaxSpeed))
  (if (Variables|Default|GetIsRunning)
    (Variables|Default|SetMaxSpeed 1e+03)
    (else
      (Variables|Default|SetMaxSpeed 6e+02))))