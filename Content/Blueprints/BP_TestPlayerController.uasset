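; BP_TestPlayerController is a player controller that lets a player without a valid controlled pawn request a respawn.
; The Respawn input action calls RequestGMRespawn only when no valid pawn is controlled.
; That event proceeds only with authority, casts the game mode to BP_TestGameMode and calls its Respawn, passing the controller itself.
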(event Custom|RequestGMRespawn
  (bind _returnvalue (Game|GetGameMode))
  (Networking|SwitchHasAuthority
    (:Authority
      (Utilities|IsValid _returnvalue
        (:Is%20Valid
          (bind _asbp_test_game_mode (Utilities|Casting|CastToBP_TestGameMode _returnvalue))
          (Utilities|IsValid _asbp_test_game_mode
            (:Is%20Valid
              (Default|Respawn _asbp_test_game_mode self))))))))

(event Input|ActionEvents|InputActionRespawn
  (params (Key :type Key%20Structure))
  (:Pressed
    (Utilities|IsValid (Pawn|GetControlledPawn self)
      (:Is%20Not%20Valid
        (CallFunction|RequestGMRespawn)))))

(fn ConstructionScript)